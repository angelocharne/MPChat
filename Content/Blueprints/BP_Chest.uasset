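; BP_Chest is a replicated chest that toggles open or closed each time a BP_TPC actor begins overlapping its Box.
; On the authority only, a FlipFlop alternates the Open variable on each valid overlap.
; Open's RepNotify plays the matching open or close animation once on the skeletal mesh, so the visual follows the replicated state.
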(event `self.Box.OnComponentBeginOverlap`
  (params (OverlappedComponent :type "PrimitiveComponent Object Reference") (OtherActor :type "Actor Object Reference") (OtherComp :type "PrimitiveComponent Object Reference") (OtherBodyIndex :type Integer) (bFromSweep :type Boolean) (SweepResult :type "HitResult Structure (by ref)"))
  (`/Engine/EditorBlueprintResources/ActorMacros.Switch Has Authority`
    (:`Authority`
      (cast `/Game/ThirdPerson/Blueprints/BP_TPC` OtherActor)
      (`/Engine/EditorBlueprintResources/StandardMacros.FlipFlop`
        (:`A`
          (set `self.Open?` true))
        (:`B`
          (set `self.Open?` false))))))

(fn `OnRep_Open?`
  (if (`self.Open?`)
    (`SkeletalMeshComponent.PlayAnimation` (`self.SkeletalMesh`) "/Game/Meshes/OpenChestAnim.OpenChestAnim" false)
    (else
      (`SkeletalMeshComponent.PlayAnimation` (`self.SkeletalMesh`) "/Game/Meshes/CloseChestAnim.CloseChestAnim" false))))

(fn `UserConstructionScript`)