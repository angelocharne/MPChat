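; BP_Laser is a laser actor whose Cube component can be rotated between two orientations.
; BeginPlay stores the Cube's starting world rotation as FirstRotation.
; Rotate plays a Timeline that lerps the Cube's world rotation toward NextRotate by the Alpha track.
; StopRotate halts the Timeline in place, and RotateReverse plays it backward toward the starting rotation.
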(event `self.ReceiveBeginPlay`
  (set `self.FirstRotation` (`SceneComponent.K2_GetComponentRotation` (`self.Cube`))))

(event `Rotate`
  (bind (_direction _alpha) (`Timeline|Timeline` :!label _label)
    (:`Update`
      (`SceneComponent.K2_SetWorldRotation` (`self.Cube`) (`KismetMathLibrary.RLerp` (`self.FirstRotation`) (`self.NextRotate`) _alpha) false false))))

(event `StopRotate`
  (goto _label :!via `Stop`))

(event `RotateReverse`
  (goto _label :!via `Reverse`))

(fn `UserConstructionScript`)