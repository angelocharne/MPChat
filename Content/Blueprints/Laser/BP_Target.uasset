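; Laser puzzle target that turns its light green while both of the first two lasers in BPLaser overlap it.
; After a one-second startup delay, Tick polls both overlaps, with a DoOnce that fires the green change once and resets when either is missing.
; When any listed laser ends overlap with LaserTargetPoint, the light turns red through the same MP change-light event.
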(event `self.ReceiveBeginPlay`
  (`KismetSystemLibrary.Delay` 1.0)
  (set `self.BeginPlayDelay` true))

(event `MP_ChangeLight`
  (params (Material :type "MaterialInterface Object Reference"))
  (`PrimitiveComponent.SetMaterial` (`self.Light`) 0 Material))

(event `CheckOverLapping`
  (bind _bp_laser (`self.BP_Laser`))
  ;[1 1 1] Check if All Actors Overlapping
  (if (and (`self.IsOverlappingActor` (`|GetArrayItem` _bp_laser) self) (`self.IsOverlappingActor` (`|GetArrayItem` _bp_laser 1) self))
    (`/Engine/EditorBlueprintResources/StandardMacros.DoOnce` false :!label _label
      (:`Completed`
        (`self.MP_ChangeLight` "/Game/Materials/M_Green.M_Green")))
    (else
      (goto _label :!via `Reset`))))

(event `self.ReceiveTick`
  (params (DeltaSeconds :type "Float (single-precision)"))
  (if (`self.BeginPlayDelay`)
    (`self.CheckOverLapping`)))

(event `self.LaserTargetPoint.OnComponentEndOverlap`
  (params (OverlappedComponent :type "PrimitiveComponent Object Reference") (OtherActor :type "Actor Object Reference") (OtherComp :type "PrimitiveComponent Object Reference") (OtherBodyIndex :type Integer))
  (for _array_element (`self.BP_Laser`)
    (if (== _array_element OtherActor)
      (`self.MP_ChangeLight` "/Game/Materials/M_Red.M_Red"))))

(fn `UserConstructionScript`)