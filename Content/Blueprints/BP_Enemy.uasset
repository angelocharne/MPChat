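; BP_Enemy is a multiplayer enemy that chases a randomly chosen player and self-destructs after damaging one on contact.
; After a startup delay, BeginPlay rolls a target index over the PlayerArray, and Tick repeatedly calls SimpleMoveToActor toward that pawn, retrying while it is invalid.
; A server-only sphere overlap applies damage to BP_TPC through a DoOnce, then destroys the enemy.
; OnRep_Max reissues the move and resets that DoOnce.
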(event `self.ReceiveBeginPlay`
  (`KismetSystemLibrary.Delay` 6.0)
  (set `self.BeginPlayDelay` true)
  (for (_ _array_index) (`GameStateBase.PlayerArray` (`GameplayStatics.GetGameState`))
    (set `self.Max` (`KismetMathLibrary.RandomIntegerInRange` 0 _array_index))))

(event `FollowPlayer`
  (bind _returnvalue (`GameplayStatics.GetPlayerPawn` (`self.Max`)))
  (`/Engine/EditorBlueprintResources/StandardMacros.IsValid` _returnvalue :!label _label
    (:`Is Valid`
      (`AIBlueprintHelperLibrary.SimpleMoveToActor` (`self.GetController`) _returnvalue))
    (:`Is Not Valid`
      (`KismetSystemLibrary.Delay` 2.0)
      (goto _label))))

(event `self.ReceiveTick`
  (params (DeltaSeconds :type "Float (single-precision)"))
  (if (`self.BeginPlayDelay`)
    (`self.FollowPlayer`)))

(event `self.Sphere.OnComponentBeginOverlap`
  (params (OverlappedComponent :type "PrimitiveComponent Object Reference") (OtherActor :type "Actor Object Reference") (OtherComp :type "PrimitiveComponent Object Reference") (OtherBodyIndex :type Integer) (bFromSweep :type Boolean) (SweepResult :type "HitResult Structure (by ref)"))
  (`/Engine/EditorBlueprintResources/ActorMacros.Switch Has Authority`
    (:`Authority`
      (bind _asbp_tpc (cast `/Game/ThirdPerson/Blueprints/BP_TPC` OtherActor))
      (`/Engine/EditorBlueprintResources/StandardMacros.DoOnce` false :!label _label_2
        (:`Completed`
          (`/Game/ThirdPerson/Blueprints/BP_TPC.SetHealth` _asbp_tpc -25.0)
          (`KismetSystemLibrary.Delay` 0.2)
          (`self.K2_DestroyActor`)
          (`self.ResetIt`))))))

(event `ResetIt`
  (goto _label_2 :!via `Reset`))

(fn `OnRep_Max`
  (bind _returnvalue (`GameplayStatics.GetPlayerPawn` (`self.Max`)))
  (if (>= (`self.Max`) 1)
    (`AIBlueprintHelperLibrary.SimpleMoveToActor` (`self.GetController`) _returnvalue)
    (else
      (`AIBlueprintHelperLibrary.SimpleMoveToActor` (`self.GetController`) _returnvalue)))
  (`self.ResetIt`))

(fn `UserConstructionScript`)