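; Two-button door puzzle that opens while BP_TPC characters occupy both trigger boxes and closes when either is left.
; Authority-only begin overlaps set the button flags, while end overlaps clear them without an authority check, with DoOnce gates throttling repeats.
; A timeline lerps the door from its start location to a Billboard marker or reverses it.
; MP_SetLight swaps the indicator light's material, green on opening and red on closing.
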(event `MP_SetLight`
  (params (Material :type "MaterialInterface Object Reference"))
  (`self.SwapColor` Material))

(event `self.ReceiveBeginPlay`
  (set `self.FirstLocation` (`SceneComponent.K2_GetComponentLocation` (`self.Door`))))

(event `OpenDoor`
  (if (and (`self.Button1Clicked?`) (`self.Button2Clicked?`))
    (`self.MP_SetLight` "/Game/Materials/M_Green.M_Green")
    (bind (_direction _alpha) (`Timeline|MoveDoor` :!label _label)
      (:`Update`
        (`SceneComponent.K2_SetWorldLocation` (`self.Door`) (`KismetMathLibrary.VLerp` (`self.FirstLocation`) (`SceneComponent.K2_GetComponentLocation` (`self.Billboard`)) _alpha) false false)))))

(event `CloseDoor`
  (`self.MP_SetLight` "/Game/Materials/M_Red.M_Red")
  (goto _label :!via `Reverse`))

(event `self.Box.OnComponentBeginOverlap`
  (params (OverlappedComponent :type "PrimitiveComponent Object Reference") (OtherActor :type "Actor Object Reference") (OtherComp :type "PrimitiveComponent Object Reference") (OtherBodyIndex :type Integer) (bFromSweep :type Boolean) (SweepResult :type "HitResult Structure (by ref)"))
  (`/Engine/EditorBlueprintResources/ActorMacros.Switch Has Authority`
    (:`Authority`
      (cast `/Game/ThirdPerson/Blueprints/BP_TPC` OtherActor)
      (`/Engine/EditorBlueprintResources/StandardMacros.DoOnce` false :!label _label_2
        (:`Completed`
          (set `self.Button1Clicked?` true)
          (`self.OpenDoor`)
          (`KismetSystemLibrary.Delay` 1.0)
          (goto _label_2 :!via `Reset`))))))

(event `self.Box1.OnComponentBeginOverlap`
  (params (OverlappedComponent :type "PrimitiveComponent Object Reference") (OtherActor :type "Actor Object Reference") (OtherComp :type "PrimitiveComponent Object Reference") (OtherBodyIndex :type Integer) (bFromSweep :type Boolean) (SweepResult :type "HitResult Structure (by ref)"))
  (`/Engine/EditorBlueprintResources/ActorMacros.Switch Has Authority`
    (:`Authority`
      (cast `/Game/ThirdPerson/Blueprints/BP_TPC` OtherActor)
      (`/Engine/EditorBlueprintResources/StandardMacros.DoOnce` false :!label _label_3
        (:`Completed`
          (set `self.Button2Clicked?` true)
          (`self.OpenDoor`)
          (`KismetSystemLibrary.Delay` 1.0)
          (goto _label_3 :!via `Reset`))))))

(event `self.Box1.OnComponentEndOverlap`
  (params (OverlappedComponent :type "PrimitiveComponent Object Reference") (OtherActor :type "Actor Object Reference") (OtherComp :type "PrimitiveComponent Object Reference") (OtherBodyIndex :type Integer))
  (cast `/Game/ThirdPerson/Blueprints/BP_TPC` OtherActor)
  (set `self.Button2Clicked?` false)
  (`/Engine/EditorBlueprintResources/StandardMacros.DoOnce` false :!label _label_4
    (:`Completed`
      (`self.CloseDoor`)
      (`KismetSystemLibrary.Delay` 0.2)
      (goto _label_4 :!via `Reset`))))

(event `self.Box.OnComponentEndOverlap`
  (params (OverlappedComponent :type "PrimitiveComponent Object Reference") (OtherActor :type "Actor Object Reference") (OtherComp :type "PrimitiveComponent Object Reference") (OtherBodyIndex :type Integer))
  (cast `/Game/ThirdPerson/Blueprints/BP_TPC` OtherActor)
  (set `self.Button1Clicked?` false)
  (goto _label_4))

(fn `SwapColor`
  (params (Material :type "MaterialInterface Object Reference"))
  (`PrimitiveComponent.SetMaterial` (`self.Light`) 0 Material))

(fn `UserConstructionScript`)