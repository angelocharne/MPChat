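; BP_Item is a pickup whose item type (Ammo, Health or Sprintboost) selects its mesh in the construction script.
; On overlap, the server disables it and starts a timer to re-enable it three seconds later.
; Only Health has an effect, calling SetHealth on an overlapping BP_TPC; the cast follows the disabling, so any overlapping actor triggers the cooldown.
; A RepNotify on Disable hides and shows the mesh.
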(event `self.StaticMesh.OnComponentBeginOverlap`
  (params (OverlappedComponent :type "PrimitiveComponent Object Reference") (OtherActor :type "Actor Object Reference") (OtherComp :type "PrimitiveComponent Object Reference") (OtherBodyIndex :type Integer) (bFromSweep :type Boolean) (SweepResult :type "HitResult Structure (by ref)"))
  (`/Engine/EditorBlueprintResources/ActorMacros.Switch Has Authority`
    (:`Authority`
      (if (not (`self.Disable?`))
        (set `self.Disable?` true)
        (`KismetSystemLibrary.K2_SetTimerDelegate` (delegate `ResetDisbale`) 3.0)
        (switch `/Game/Blueprints/E_Item` (`self.ItemTyp`)
          (:`NewEnumerator1`
            (bind _asbp_tpc (cast `/Game/ThirdPerson/Blueprints/BP_TPC` OtherActor))
            (`/Game/ThirdPerson/Blueprints/BP_TPC.SetHealth` _asbp_tpc 25.0)))))))

(event `ResetDisbale`
  (set `self.Disable?` false))

(fn `OnRep_Disable?`
  (`SceneComponent.SetVisibility` (`self.StaticMesh`) (not (`self.Disable?`)) false))

(fn `UserConstructionScript`
  (bind _staticmesh (`self.StaticMesh`))
  (switch `/Game/Blueprints/E_Item` (`self.ItemTyp`)
    (:`NewEnumerator0`
      (`StaticMeshComponent.SetStaticMesh` _staticmesh "/Game/LevelPrototyping/Meshes/SM_Cylinder.SM_Cylinder"))
    (:`NewEnumerator1`
      (`StaticMeshComponent.SetStaticMesh` _staticmesh "/Game/LevelPrototyping/Meshes/SM_ChamferCube.SM_ChamferCube"))
    (:`NewEnumerator2`
      (`StaticMeshComponent.SetStaticMesh` _staticmesh "/Game/LevelPrototyping/Meshes/SM_Ramp.SM_Ramp"))))