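; Lobby player controller for multiplayer that opens the lobby widget with mouse cursor and UI-only input on BeginPlay.
; It reads the nickname from MPGameInstance and passes it to SetNicknameToServer.
; Server-named events send nickname-prefixed chat and player status changes to BP_GameMode for distribution.
; AddMessage and ClientUpdatePlayerList feed chat and player lists into the widget; a nickname debug-print timer is left disconnected.
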(event `LocalePlayerName`
  (`KismetSystemLibrary.PrintText` (`|FormatText` "Client : {Nickname} " (`self.Nickname`))))

(event `self.ReceiveBeginPlay`
  (bind _returnvalue (`|CreateWidget` "/Game/Blueprints/UI/WBP_Lobby.WBP_Lobby_C" (`GameplayStatics.GetPlayerController` 0)))
  (bind _output_get (set `self.WBP_Chat` _returnvalue))
  (`UserWidget.AddToViewport` _output_get 0)
  (`WidgetBlueprintLibrary.SetInputMode_UIOnlyEx` self (`self.WBP_Chat`))
  (set `self.bShowMouseCursor` true)
  (`self.GetAndSaveNicknameFromGameInsatnce`))

(event `GetAndSaveNicknameFromGameInsatnce`
  (bind _asmpgame_instance (cast `/Game/Game/MPGameInstance` (`GameplayStatics.GetGameInstance`)))
  (`self.SetNicknametoServer` (`/Game/Game/MPGameInstance.Nickname` _asmpgame_instance)))

(event `SetNicknameToServer`
  (params (Nickname :type Text))
  (set `self.Nickname` Nickname))

(event `ServerSendMessage`
  (params (Message :type Text))
  (bind _asbp_game_mode (cast `/Game/Game/BP_GameMode` (`GameplayStatics.GetGameMode`)))
  (`/Game/Game/BP_GameMode.SendMessageToAll` _asbp_game_mode (`|FormatText` "{Nickname} : {Message} " (`self.Nickname`) Message)))

(event `ServerSetMyPlayerStatus`
  (params (PlayerStruct :type "/Game/Blueprints/S_Player Structure"))
  (set `self.PlayerStruct` PlayerStruct)
  (bind _asbp_game_mode (cast `/Game/Game/BP_GameMode` (`GameplayStatics.GetGameMode`)))
  (`/Game/Game/BP_GameMode.SendUptaeUI ToClient` _asbp_game_mode))

(event `AddMessage`
  (params (Message :type Text))
  (`/Game/Blueprints/UI/WBP_Lobby.AddMessageToScrollBox` (`self.WBP_Chat`) Message))

(event `ClientUpdatePlayerList`
  (params (PlayerInfo :type "Array of /Game/Blueprints/S_Player Structure (by ref)"))
  (`/Game/Blueprints/UI/WBP_Lobby.RefreshPlayerList` (`self.WBP_Chat`) PlayerInfo))

(fn `UserConstructionScript`)