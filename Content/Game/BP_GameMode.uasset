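; Lobby game mode Blueprint that tracks joined players and relays chat and player-list updates to them.
; PostLogin adds each BP_LobbyPlayerController to an array that the broadcast events loop over.
; SendMessageToAll pushes a message to every controller, while SendUptaeUIToClient rebuilds the player info list from their PlayerStructs and sends it to each client.
; A looping server timer prints every stored nickname, apparently for debugging.
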(event `self.ReceiveBeginPlay`
  (`/Engine/EditorBlueprintResources/ActorMacros.Switch Has Authority`
    (:`Authority`
      (`KismetSystemLibrary.K2_SetTimerDelegate` (delegate `TestPlayername`) 2.0 true))))

(event `TestPlayername`
  (for _array_element (`self.AllPlayerControllerChat`)
    (`KismetSystemLibrary.PrintText` (`/Game/Game/BP_LobbyPlayerController.Nickname` _array_element))))

(event `self.K2_PostLogin`
  (params (NewPlayer :type "PlayerController Object Reference"))
  (bind _asbp_lobby_player_controller (cast `/Game/Game/BP_LobbyPlayerController` NewPlayer))
  (`KismetArrayLibrary.Array_AddUnique` (`self.AllPlayerControllerChat`) _asbp_lobby_player_controller))

(event `SendMessageToAll`
  (params (Message :type Text))
  (for _array_element (`self.AllPlayerControllerChat`)
    (`/Game/Game/BP_LobbyPlayerController.AddMessage` _array_element Message)))

(event `SendUptaeUI ToClient`
  (bind _allplayercontrollerchat (`self.AllPlayerControllerChat`))
  (`KismetArrayLibrary.Array_Clear` (`self.PlayerInfos`))
  (for _array_element _allplayercontrollerchat
    (`KismetArrayLibrary.Array_AddUnique` (`self.PlayerInfos`) (`/Game/Game/BP_LobbyPlayerController.PlayerStruct` _array_element)))
  (for _array_element_2 _allplayercontrollerchat
    (`/Game/Game/BP_LobbyPlayerController.ClientUpdatePlayerList` _array_element_2 (`self.PlayerInfos`))))

(fn `UserConstructionScript`)