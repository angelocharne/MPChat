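; BP_LevelPlayerController is the player controller for a level, setting up the local player's HUD and stats overlay.
; On BeginPlay, for the local controller only, it clears existing widgets, switches to game-only input, and adds the in-game HUD plus a hidden player stats widget.
; Holding the ShowStats input refreshes and shows the stats widget, and releasing it hides the widget again.
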(event `self.ReceiveBeginPlay`
  (if (`self.IsLocalPlayerController`)
    (`WidgetLayoutLibrary.RemoveAllWidgets`)
    (`WidgetBlueprintLibrary.SetInputMode_GameOnly` self)
    (bind _returnvalue (`|CreateWidget` "/Game/Blueprints/UI/WBP_InGameHUD.WBP_InGameHUD_C"))
    (`UserWidget.AddToViewport` _returnvalue 0)
    (bind _returnvalue_2 (`|CreateWidget` "/Game/Blueprints/UI/WBP_PlayerStats.WBP_PlayerStats_C"))
    (bind _output_get (set `self.Stats` _returnvalue_2))
    (`Widget.SetVisibility` _returnvalue_2 "Hidden")
    (`Widget.SetVisibility` _output_get "Hidden")
    (`UserWidget.AddToViewport` _output_get 0)))

(event `self.ReceiveTick`
  (params (DeltaSeconds :type "Float (single-precision)")))

(event `InputAction|ShowStats`
  (params (Key :type "Key Structure"))
  (bind _stats (`self.Stats`))
  (:`Pressed`
    (`/Game/Blueprints/UI/WBP_PlayerStats.RefreshStats` _stats)
    (`Widget.SetVisibility` _stats "Visible"))
  (:`Released`
    (`Widget.SetVisibility` _stats "Hidden")))

(fn `UserConstructionScript`)