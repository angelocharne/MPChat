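; Level game mode that carries lobby players into the match, spawns their colored BP_TPC characters and respawns them on death.
; OnSwapPlayerControllers copies lobby player data to each level controller, registers it and sets the nickname.
; BeginPlay spawns and possesses pawns at PlayerStarts tagged by player index, stepping the GameState's GameStatus through three timed phases.
; Authority Tick polls and prints health, respawning any pawn at zero at its indexed start.
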(event `self.ReceiveBeginPlay`
  (`KismetSystemLibrary.Delay` 0.2)
  (bind _asbp_game_state_level (cast `/Game/Game/Level/BP_GameStateLevel` (`GameplayStatics.GetGameState`)))
  (set `/Game/Game/Level/BP_GameStateLevel.GameStatus` "NewEnumerator0" _asbp_game_state_level)
  (`self.SpawnPlayersAndPosses`)
  (`KismetSystemLibrary.Delay` 4.0)
  (set `/Game/Game/Level/BP_GameStateLevel.GameStatus` "NewEnumerator1" _asbp_game_state_level)
  (`KismetSystemLibrary.Delay` 3.0)
  (set `/Game/Game/Level/BP_GameStateLevel.GameStatus` "NewEnumerator2" _asbp_game_state_level))

(event `SpawnPlayersAndPosses`
  (for (_array_element _array_index) (`self.AllPlayerController`)
    (bind _returnvalue (`Controller.K2_GetPawn` _array_element))
    (`/Engine/EditorBlueprintResources/StandardMacros.IsValid` _returnvalue
      (:`Is Valid`
        (`self.K2_DestroyActor` _returnvalue))
      (:`Is Not Valid`
        _))
    (bind _pos (`self.GetPlayerStartsLocaton` _array_index))
    (bind (_playerstatus_playername _playerstatus_isready_ _playerstatus_color _playerstatus_linearcolor) (break `/Game/Blueprints/S_Player` (`/Game/Game/Level/BP_LevelPlayerController.PlayerStatus` _array_element)))
    (bind _returnvalue_2 (`|SpawnActorFromClass` "/Game/ThirdPerson/Blueprints/BP_TPC.BP_TPC_C" (`KismetMathLibrary.MakeTransform` _pos) "Undefined" "OverrideRootScale" null _playerstatus_linearcolor null))
    (`Controller.Possess` _array_element _returnvalue_2)))

(event `self.ReceiveTick`
  (params (DeltaSeconds :type "Float (single-precision)"))
  (`/Engine/EditorBlueprintResources/ActorMacros.Switch Has Authority`
    (:`Authority`
      (`self.CheckHealth`))))

(event `self.K2_OnSwapPlayerControllers`
  (params (OldPC :type "PlayerController Object Reference") (NewPC :type "PlayerController Object Reference"))
  ;[1 1 1] Event On SwapPlayerController
  (bind _asbp_lobby_player_controller (cast `/Game/Game/BP_LobbyPlayerController` OldPC))
  (bind _asbp_level_player_controller (cast `/Game/Game/Level/BP_LevelPlayerController` NewPC))
  (bind _output_get (set `/Game/Game/Level/BP_LevelPlayerController.PlayerStatus` (`/Game/Game/BP_LobbyPlayerController.PlayerStruct` _asbp_lobby_player_controller) _asbp_level_player_controller))
  (`KismetArrayLibrary.Array_AddUnique` (`self.AllPlayerController`) _asbp_level_player_controller)
  (bind _asbp_level_player_state (cast `/Game/Game/Level/BP_LevelPlayerState` (`Controller.PlayerState` _asbp_level_player_controller)))
  (set `/Game/Game/Level/BP_LevelPlayerState.Nickname` (`KismetTextLibrary.Conv_TextToString` (`.PlayerName_2_F45B171B458565E14DA4069385A1E570` (break `/Game/Blueprints/S_Player` _output_get))) _asbp_level_player_state))

(event `self.K2_PostLogin`
  (params (NewPlayer :type "PlayerController Object Reference"))
  ;[1 0 0] Debug Check
)

(fn `CheckHealth`
  (for (_array_element _array_index) (`self.AllPlayerController`)
    (bind _asbp_tpc (cast `/Game/ThirdPerson/Blueprints/BP_TPC` (`Controller.K2_GetPawn` _array_element)))
    (bind _health (`/Game/ThirdPerson/Blueprints/BP_TPC.Health` _asbp_tpc))
    (`KismetSystemLibrary.PrintString` (`KismetStringLibrary.Conv_DoubleToString` _health))
    (if (<= _health 0.0)
      (`self.K2_DestroyActor` _asbp_tpc)
      (bind _pos (`self.GetPlayerStartsLocaton` _array_index))
      (bind (_playerstatus_playername _playerstatus_isready_ _playerstatus_color _playerstatus_linearcolor) (break `/Game/Blueprints/S_Player` (`/Game/Game/Level/BP_LevelPlayerController.PlayerStatus` _array_element)))
      (bind _returnvalue (`|SpawnActorFromClass` "/Game/ThirdPerson/Blueprints/BP_TPC.BP_TPC_C" (`KismetMathLibrary.MakeTransform` _pos) "Undefined" "OverrideRootScale" null _playerstatus_linearcolor null))
      (`Controller.Possess` _array_element _returnvalue))))

(fn `GetPlayerStartsLocaton`
  (params (Index :type Integer))
  (returns (Pos :type "Vector Structure"))
  (bind _outactors (`GameplayStatics.GetAllActorsOfClass` "/Script/Engine.PlayerStart"))
  (for _array_element _outactors
    (if (== (`PlayerStart.PlayerStartTag` _array_element) (`KismetStringLibrary.Conv_StringToName` (`KismetStringLibrary.Conv_IntToString` Index)))
      (return (`self.K2_GetActorLocation` _array_element)))))

(fn `UserConstructionScript`)